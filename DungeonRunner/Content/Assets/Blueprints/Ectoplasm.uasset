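; Ectoplasm is a hazard actor that kills the player character on overlap.
; Overlap plays a damage sound, sets the ThirdPersonCharacter's HitByEctoplasm flag, calls its DeathFunction and toggles mesh visibility.
; After a short delay it clears the flag on player 0's character and destroys itself.
; A Delay on Tick also destroys it after a fixed lifetime.
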(event EventBeginPlay)

(event Collision|EventActorBeginOverlap
  (params (OtherActor :type Actor%20Object%20Reference))
  ;[1 1 1] on collison with player, Call Death Function, destroy itself
  (bind _asthird_person_character (Utilities|Casting|CastToThirdPersonCharacter OtherActor))
  (Audio|PlaySound2D "/Game/Sounds/take_damage.take_damage" 1.0 1.0 0.0 0 0)
  (Variables|/Game/UE4_Content/ThirdPersonBP/Blueprints/ThirdPersonCharacter.ThirdPersonCharacter_C|SetHitByEctoplasm _asthird_person_character true)
  (Default|DeathFunction _asthird_person_character)
  (Rendering|ToggleVisibility (Variables|Default|GetStaticMesh) false)
  (Utilities|FlowControl|Delay 0.5)
  (bind _asthird_person_character_2 (Utilities|Casting|CastToThirdPersonCharacter (Game|GetPlayerCharacter 0)))
  (Variables|/Game/UE4_Content/ThirdPersonBP/Blueprints/ThirdPersonCharacter.ThirdPersonCharacter_C|SetHitByEctoplasm _asthird_person_character_2 false)
  (Actor|DestroyActor))

(event EventTick
  (params (DeltaSeconds :type Float%20%28single-precision%29))
  ;[1 1 1] Destroy itself on timer
  (Utilities|FlowControl|Delay 35.0)
  (Actor|DestroyActor))

(fn ConstructionScript)