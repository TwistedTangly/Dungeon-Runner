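; Enemy actor that kills the player on touch and periodically spawns Ectoplasm projectiles.
; It plays a bat sound on BeginPlay, and overlapping a ThirdPersonCharacter calls that character's DeathFunction and destroys the enemy.
; Chained Delay nodes on Tick act as timers, repeatedly spawning Ectoplasm at the Spawn component's transform and destroying the enemy about 40 seconds after it starts.
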(event EventBeginPlay
  (Audio|PlaySoundatLocation "/Game/Sounds/enemy_bats.enemy_bats" (Transformation|GetActorLocation) "0, 0, 0" 1.0 1.0 0.0 0 0 0))

(event Collision|EventActorBeginOverlap
  (params (OtherActor :type Actor%20Object%20Reference))
  ;[1 1 1] If player collides,call death function, destroy actor
  (bind _asthird_person_character (Utilities|Casting|CastToThirdPersonCharacter OtherActor))
  (Default|DeathFunction _asthird_person_character)
  (Actor|DestroyActor))

(event EventTick
  (params (DeltaSeconds :type Float%20%28single-precision%29))
  ;[1 1 1] Spawn projectile on timer
  (Utilities|FlowControl|Delay 5.0)
  (Game|SpawnActorfromClass "/Game/Assets/Blueprints/Ectoplasm.Ectoplasm_C" (Transformation|GetWorldTransform (Variables|Default|GetSpawn)) "Undefined" 0 0)
  (Utilities|FlowControl|Delay 35.0)
  (Actor|DestroyActor))

(fn ConstructionScript)