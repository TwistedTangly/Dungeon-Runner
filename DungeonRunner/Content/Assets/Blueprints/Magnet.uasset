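; Magnet power-up pickup that temporarily switches on the third-person character's magnet when overlapped.
; Pickup plays a sound, shows the character's Magnet, sets MagnetActive and hides itself, then reverts both after ten seconds and destroys itself.
; If the character already has a magnet or sword, it awards bonus GameMode coins instead.
; A Delay on Tick destroys the actor 35 seconds into its life, even mid-effect.
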(event EventBeginPlay)

(event Collision|EventActorBeginOverlap
  (params (OtherActor :type Actor%20Object%20Reference))
  ;[1 1 1] Set magent Active, disable visability
  (bind _asthird_person_character (Utilities|Casting|CastToThirdPersonCharacter OtherActor))
  (Audio|PlaySound2D "/Game/Sounds/special_pickup.special_pickup" 1.0 1.0 0.0 0 0)
  (if (Variables|/Game/UE4_Content/ThirdPersonBP/Blueprints/ThirdPersonCharacter.ThirdPersonCharacter_C|GetMagnetActive _asthird_person_character)
    (bind _asthird_person_game_mode (Utilities|Casting|CastToThirdPersonGameMode (Game|GetGameMode) :!label _label))
    (Variables|/Game/UE4_Content/ThirdPersonBP/Blueprints/ThirdPersonGameMode.ThirdPersonGameMode_C|SetCoins _asthird_person_game_mode (+ (Variables|/Game/UE4_Content/ThirdPersonBP/Blueprints/ThirdPersonGameMode.ThirdPersonGameMode_C|GetCoins _asthird_person_game_mode) 20))
    (Actor|DestroyActor)
    (elif (Variables|/Game/UE4_Content/ThirdPersonBP/Blueprints/ThirdPersonCharacter.ThirdPersonCharacter_C|GetHas%20Sword _asthird_person_character)
      (goto _label)
      (else
        (Rendering|ToggleVisibility (Variables|/Game/UE4_Content/ThirdPersonBP/Blueprints/ThirdPersonCharacter.ThirdPersonCharacter_C|GetMagnet _asthird_person_character) false)
        (Variables|/Game/UE4_Content/ThirdPersonBP/Blueprints/ThirdPersonCharacter.ThirdPersonCharacter_C|SetMagnetActive _asthird_person_character true)
        (Development|PrintString "Mag On")
        (Rendering|SetVisibility (Variables|Default|GetPickup) false false)
        ;[1 1 1] Set magnet off, Destroy actor after timer
        (Utilities|FlowControl|Delay 1e+01)
        (bind _asthird_person_character_2 (Utilities|Casting|CastToThirdPersonCharacter (Game|GetPlayerCharacter 0)))
        (Rendering|ToggleVisibility (Variables|/Game/UE4_Content/ThirdPersonBP/Blueprints/ThirdPersonCharacter.ThirdPersonCharacter_C|GetMagnet _asthird_person_character_2) false)
        (Variables|/Game/UE4_Content/ThirdPersonBP/Blueprints/ThirdPersonCharacter.ThirdPersonCharacter_C|SetMagnetActive _asthird_person_character_2 false)
        (Development|PrintString "Mag Off")
        (Actor|DestroyActor)))))

(event EventTick
  (params (DeltaSeconds :type Float%20%28single-precision%29))
  ;[1 1 1] Destroy actor on timer
  (Utilities|FlowControl|Delay 35.0)
  (Actor|DestroyActor))

(fn ConstructionScript)