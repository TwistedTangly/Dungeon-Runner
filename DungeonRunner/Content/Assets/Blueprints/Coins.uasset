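; Coin pickup that adds to the game mode's coin count when the player character touches it, and destroys itself after 35 seconds.
; An outer Sphere overlap checks the character's magnet; if active, it credits the coin immediately, slides it toward the player via timeline and VInterpTo, then destroys it shortly after.
; The inner Pickup overlap plays a sound and collects the coin, with a Used flag preventing double counting.
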(event OnComponentBeginOverlap(Sphere)
  (params (OverlappedComponent :type Primitive%20Component%20Object%20Reference) (OtherActor :type Actor%20Object%20Reference) (OtherComp :type Primitive%20Component%20Object%20Reference) (OtherBodyIndex :type Integer) (bFromSweep :type Boolean) (SweepResult :type Hit%20Result%20Structure%20%28by%20ref%29))
  ;[1 1 1] On ovewrlap with sphere collision with magnet active
  (bind _asthird_person_character (Utilities|Casting|CastToThirdPersonCharacter OtherActor))
  (if (Variables|/Game/UE4_Content/ThirdPersonBP/Blueprints/ThirdPersonCharacter.ThirdPersonCharacter_C|GetMagnetActive _asthird_person_character)
    (Utilities|FlowControl|Sequence
      (:then_0
        (bind _asthird_person_game_mode (Utilities|Casting|CastToThirdPersonGameMode (Game|GetGameMode)))
        (Math|Integer|IncrementInt (Variables|/Game/UE4_Content/ThirdPersonBP/Blueprints/ThirdPersonGameMode.ThirdPersonGameMode_C|GetCoins _asthird_person_game_mode)
          (:%20%20
            (Variables|Default|SetUsed true)
            (Utilities|FlowControl|Delay 0.2)
            (Actor|DestroyActor))))
      (:then_1
        (bind _slide (Timeline|Timeline_0 Play)
          (:Update
            (Transformation|SetActorLocation (+ _slide (Math|Interpolation|VInterpTo (.Location (Math|Transform|BreakTransform (Transformation|GetActorTransform))) (Transformation|GetActorLocation (Game|GetPlayerCharacter 0)) (Utilities|Time|GetWorldDeltaSeconds) 15.0)) false false)))))))

(event OnComponentBeginOverlap(Pickup)
  (params (OverlappedComponent :type Primitive%20Component%20Object%20Reference) (OtherActor :type Actor%20Object%20Reference) (OtherComp :type Primitive%20Component%20Object%20Reference) (OtherBodyIndex :type Integer) (bFromSweep :type Boolean) (SweepResult :type Hit%20Result%20Structure%20%28by%20ref%29))
  ;[1 1 1] On Overlap with coin add to gold and destroy
  (Utilities|Casting|CastToThirdPersonCharacter OtherActor)
  (Audio|PlaySound2D "/Game/Sounds/coin/CoinCue.CoinCue" 1.0 1.0 0.0 0 0)
  (bind _asthird_person_game_mode (Utilities|Casting|CastToThirdPersonGameMode (Game|GetGameMode)))
  (if (not (Variables|Default|GetUsed))
    (Math|Integer|IncrementInt (Variables|/Game/UE4_Content/ThirdPersonBP/Blueprints/ThirdPersonGameMode.ThirdPersonGameMode_C|GetCoins _asthird_person_game_mode)
      (:%20%20
        (Actor|DestroyActor)))))

(event EventBeginPlay)

(event EventTick
  (params (DeltaSeconds :type Float%20%28single-precision%29))
  ;[1 1 1] Destroy on timer
  (Utilities|FlowControl|Delay 35.0)
  (Actor|DestroyActor))

(fn ConstructionScript)