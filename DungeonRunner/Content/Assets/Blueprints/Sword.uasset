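; Sword pickup that temporarily equips the third-person character with a sword when overlapped.
; If the character already has a sword or an active magnet, it instead adds coins through ThirdPersonGameMode and destroys itself.
; Otherwise it toggles the character's Sword visibility, sets HasSword and hides the pickup, then reverses this after a delay and destroys itself.
; A separate Delay on Tick also destroys the actor, regardless of pickup state.
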(event EventBeginPlay)

(event Collision|EventActorBeginOverlap
  (params (OtherActor :type Actor%20Object%20Reference))
  ;[1 1 1] Set the sword active, Set vissibilty off
  (bind _asthird_person_character (Utilities|Casting|CastToThirdPersonCharacter OtherActor))
  (if (Variables|/Game/UE4_Content/ThirdPersonBP/Blueprints/ThirdPersonCharacter.ThirdPersonCharacter_C|GetHas%20Sword _asthird_person_character)
    (bind _asthird_person_game_mode (Utilities|Casting|CastToThirdPersonGameMode (Game|GetGameMode) :!label _label))
    (Variables|/Game/UE4_Content/ThirdPersonBP/Blueprints/ThirdPersonGameMode.ThirdPersonGameMode_C|SetCoins _asthird_person_game_mode (+ (Variables|/Game/UE4_Content/ThirdPersonBP/Blueprints/ThirdPersonGameMode.ThirdPersonGameMode_C|GetCoins _asthird_person_game_mode) 20))
    (Actor|DestroyActor)
    (elif (Variables|/Game/UE4_Content/ThirdPersonBP/Blueprints/ThirdPersonCharacter.ThirdPersonCharacter_C|GetMagnetActive _asthird_person_character)
      (goto _label)
      (else
        (Rendering|ToggleVisibility (Variables|/Game/UE4_Content/ThirdPersonBP/Blueprints/ThirdPersonCharacter.ThirdPersonCharacter_C|GetSword _asthird_person_character) false)
        (Variables|/Game/UE4_Content/ThirdPersonBP/Blueprints/ThirdPersonCharacter.ThirdPersonCharacter_C|SetHas%20Sword _asthird_person_character true)
        (Development|PrintString "Sword On")
        (Rendering|SetVisibility (Variables|Default|GetPickup) false false)
        ;[1 1 1] After delay turn of sword , destroy actor
        (Utilities|FlowControl|Delay 1e+01)
        (bind _asthird_person_character_2 (Utilities|Casting|CastToThirdPersonCharacter (Game|GetPlayerCharacter 0)))
        (Rendering|ToggleVisibility (Variables|/Game/UE4_Content/ThirdPersonBP/Blueprints/ThirdPersonCharacter.ThirdPersonCharacter_C|GetSword _asthird_person_character_2) false)
        (Variables|/Game/UE4_Content/ThirdPersonBP/Blueprints/ThirdPersonCharacter.ThirdPersonCharacter_C|SetHas%20Sword _asthird_person_character_2 false)
        (Development|PrintString "Sword Broke")
        (Actor|DestroyActor)))))

(event EventTick
  (params (DeltaSeconds :type Float%20%28single-precision%29))
  ;[1 1 1] Destroy Actor on timer
  (Utilities|FlowControl|Delay 35.0)
  (Actor|DestroyActor))

(fn ConstructionScript)