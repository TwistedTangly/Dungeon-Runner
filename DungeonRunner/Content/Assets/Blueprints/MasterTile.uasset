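; MasterTile is a track tile for a three-lane endless runner that spawns its own obstacles on BeginPlay.
; SpawnObstacles randomly picks rocks, barrels, side walls or nothing, rolling the middle lane only after left-lane rocks and the right only after middle-lane rocks.
; When the player overlaps its Box, it asks the game mode for another tile, adds multiplied score, slightly raises clamped walk speed, then destroys itself after a delay.
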(event OnComponentBeginOverlap(Box)
  (params (OverlappedComponent :type Primitive%20Component%20Object%20Reference) (OtherActor :type Actor%20Object%20Reference) (OtherComp :type Primitive%20Component%20Object%20Reference) (OtherBodyIndex :type Integer) (bFromSweep :type Boolean) (SweepResult :type Hit%20Result%20Structure%20%28by%20ref%29))
  (Utilities|Casting|CastToThirdPersonCharacter OtherActor)
  (bind _asthird_person_game_mode (Utilities|Casting|CastToThirdPersonGameMode (Game|GetGameMode)))
  (Default|SpawnTile _asthird_person_game_mode)
  (bind _asthird_person_game_mode_2 (Utilities|Casting|CastToThirdPersonGameMode (Game|GetGameMode)))
  (Variables|/Game/UE4_Content/ThirdPersonBP/Blueprints/ThirdPersonGameMode.ThirdPersonGameMode_C|SetCurrentScore _asthird_person_game_mode_2 (+ (* 1 (Variables|/Game/UE4_Content/ThirdPersonBP/Blueprints/ThirdPersonGameMode.ThirdPersonGameMode_C|GetScoreMultiplier _asthird_person_game_mode_2)) (Variables|/Game/UE4_Content/ThirdPersonBP/Blueprints/ThirdPersonGameMode.ThirdPersonGameMode_C|GetCurrentScore _asthird_person_game_mode_2)))
  (bind _asthird_person_character (Utilities|Casting|CastToThirdPersonCharacter (Game|GetPlayerCharacter 0)))
  (Variables|/Script/Engine.CharacterMovementComponent|SetMaxWalkSpeed (Variables|/Script/Engine.Character|GetCharacterMovement _asthird_person_character) (Math|Float|Clamp(Float) (* (Variables|/Script/Engine.CharacterMovementComponent|GetMaxWalkSpeed (Variables|/Script/Engine.Character|GetCharacterMovement _asthird_person_character)) 1.01) 6e+02 1.2e+03))
  (Utilities|FlowControl|Delay 2.0)
  (Actor|DestroyActor))

(event EventBeginPlay
  (CallFunction|SpawnObstacles))

(event Collision|EventActorBeginOverlap
  (params (OtherActor :type Actor%20Object%20Reference)))

(event EventTick
  (params (DeltaSeconds :type Float%20%28single-precision%29)))

(fn ConstructionScript)

(fn SpawnObstacles
  (bind _leftlane (Variables|Default|GetLeftLane))
  (bind _middlelane (Variables|Default|GetMiddleLane))
  (bind _rightlane (Variables|Default|GetRightLane))
  (bind _returnvalue (Transformation|GetWorldTransform _rightlane))
  (bind _returnvalue_2 (Transformation|GetWorldTransform _leftlane))
  (bind _returnvalue_3 (Transformation|GetWorldTransform _middlelane))
  ;[1 1 1] Left Lane - Adding more pins to Switch allows for different objeects to spawn _More empty pins means less chance of something spawning
  (switch int (Math|Random|RandomIntegerinRange 0 3)
    (:1
      (Game|SpawnActorfromClass "/Game/Assets/Blueprints/ObstacleRocks.ObstacleRocks_C" _returnvalue_2 "Undefined" 0 0)
      ;[1 1 1] Middle Lane
      (switch int (Math|Random|RandomIntegerinRange 0 2)
        (:1
          (Game|SpawnActorfromClass "/Game/Assets/Blueprints/ObstacleRocks.ObstacleRocks_C" _returnvalue_3 "Undefined" 0 0)
          ;[1 1 1] Right Lane
          (switch int (Math|Random|RandomIntegerinRange 0 3)
            (:1
              (Game|SpawnActorfromClass "/Game/Assets/Blueprints/ObstacleRocks.ObstacleRocks_C" _returnvalue "Undefined" 0 0))
            (:2
              (Game|SpawnActorfromClass "/Game/Assets/Blueprints/ObstacleBarrel.ObstacleBarrel_C" _returnvalue "Undefined" 0 0))
            (:3
              (Game|SpawnActorfromClass "/Game/Assets/Blueprints/ObstacleWall_Right.ObstacleWall_Right_C" _returnvalue "Undefined" 0 0))))
        (:2
          (Game|SpawnActorfromClass "/Game/Assets/Blueprints/ObstacleBarrel.ObstacleBarrel_C" _returnvalue_3 "Undefined" 0 0))))
    (:2
      (Game|SpawnActorfromClass "/Game/Assets/Blueprints/ObstacleBarrel.ObstacleBarrel_C" _returnvalue_2 "Undefined" 0 0))
    (:3
      (Game|SpawnActorfromClass "/Game/Assets/Blueprints/ObstacleWall_Left.ObstacleWall_Left_C" _returnvalue_2 "Undefined" 0 0))))