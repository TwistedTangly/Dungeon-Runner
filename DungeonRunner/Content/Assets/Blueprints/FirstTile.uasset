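; Endless-runner floor tile with three lanes that can hold coins, obstacles, milk and magnets.
; Outside the main menu, player overlap of its box has the game mode spawn another tile, adds distance, raises clamped walk speed, then destroys the tile after a delay.
; SpawnObstacles, not called here, fills lanes left to right through chained range checks.
; Each check rerolls, and a lane where all fail skips any remaining lanes.
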(event OnComponentBeginOverlap(Box)
  (params (OverlappedComponent :type Primitive%20Component%20Object%20Reference) (OtherActor :type Actor%20Object%20Reference) (OtherComp :type Primitive%20Component%20Object%20Reference) (OtherBodyIndex :type Integer) (bFromSweep :type Boolean) (SweepResult :type Hit%20Result%20Structure%20%28by%20ref%29))
  (bind _asthird_person_character (Utilities|Casting|CastToThirdPersonCharacter OtherActor))
  (if (not (Variables|/Game/UE4_Content/ThirdPersonBP/Blueprints/ThirdPersonCharacter.ThirdPersonCharacter_C|GetisMainMenu _asthird_person_character))
    (bind _asthird_person_game_mode (Utilities|Casting|CastToThirdPersonGameMode (Game|GetGameMode)))
    (Default|SpawnTile _asthird_person_game_mode)
    (bind _asthird_person_game_mode_2 (Utilities|Casting|CastToThirdPersonGameMode (Game|GetGameMode)))
    (Variables|/Game/UE4_Content/ThirdPersonBP/Blueprints/ThirdPersonGameMode.ThirdPersonGameMode_C|SetDistance _asthird_person_game_mode_2 (+ (Variables|/Game/UE4_Content/ThirdPersonBP/Blueprints/ThirdPersonGameMode.ThirdPersonGameMode_C|GetDistance _asthird_person_game_mode_2) 10))
    (bind _asthird_person_character_2 (Utilities|Casting|CastToThirdPersonCharacter (Game|GetPlayerCharacter 0)))
    (Variables|/Script/Engine.CharacterMovementComponent|SetMaxWalkSpeed (Variables|/Script/Engine.Character|GetCharacterMovement _asthird_person_character_2) (Math|Float|Clamp(Float) (* (Variables|/Script/Engine.CharacterMovementComponent|GetMaxWalkSpeed (Variables|/Script/Engine.Character|GetCharacterMovement _asthird_person_character_2)) 1.01) 6e+02 1.2e+03))
    (Utilities|FlowControl|Delay 2.0)
    (Actor|DestroyActor)))

(event EventBeginPlay)

(event Collision|EventActorBeginOverlap
  (params (OtherActor :type Actor%20Object%20Reference)))

(event EventTick
  (params (DeltaSeconds :type Float%20%28single-precision%29)))

(fn ConstructionScript)

(fn SpawnObstacles
  (bind _returnvalue (Math|Random|RandomFloatinRange 0.0 1.0))
  (bind _returnvalue_2 (Math|Random|RandomFloatinRange 0.0 1.0))
  (bind _returnvalue_3 (Math|Random|RandomFloatinRange 0.0 1.0))
  (bind _leftlane (Variables|Default|GetLeftLane))
  (bind _middlelane (Variables|Default|GetMiddleLane))
  (bind _rightlane (Variables|Default|GetRightLane))
  (bind _returnvalue_4 (Transformation|GetWorldTransform _leftlane))
  (bind _returnvalue_5 (Transformation|GetWorldTransform _middlelane))
  (bind _returnvalue_6 (Transformation|GetWorldTransform _rightlane))
  ;[1 1 1] Left Lane - Range 0f 1 - changes the percentage change of those obsticles spawning dependent of selected values
  (if (Math|Float|InRange(Float) _returnvalue 0.0 0.3)
    (Game|SpawnActorfromClass "/Game/Assets/Blueprints/CoinPickup.CoinPickup_C" _returnvalue_4 "Undefined" 0 0)
    ;[1 1 1] Middle Lane
    (if (Math|Float|InRange(Float) _returnvalue_3 0.0 0.3) :!label _label
      (Game|SpawnActorfromClass "/Game/Assets/Blueprints/CoinPickup.CoinPickup_C" _returnvalue_5 "Undefined" 0 0)
      ;[1 1 1] Right Lane
      (if (Math|Float|InRange(Float) _returnvalue_2 0.0 0.3) :!label _label_2
        (Game|SpawnActorfromClass "/Game/Assets/Blueprints/CoinPickup.CoinPickup_C" _returnvalue_6 "Undefined" 0 0)
        (elif (Math|Float|InRange(Float) _returnvalue_2 0.3 0.5)
          (Game|SpawnActorfromClass "/Game/Assets/Blueprints/ObstacleBarrel.ObstacleBarrel_C" _returnvalue_6 "Undefined" 0 0)
          (Game|SpawnActorfromClass "/Game/Assets/Blueprints/CoinPickupJump.CoinPickupJump_C" _returnvalue_6 "Undefined" 0 0)
          (elif (Math|Float|InRange(Float) _returnvalue_2 0.5 0.7)
            (Game|SpawnActorfromClass "/Game/Assets/Blueprints/ObstacleBarrel.ObstacleBarrel_C" _returnvalue_6 "Undefined" 0 0)
            (elif (Math|Float|InRange(Float) _returnvalue_2 0.7 0.8)
              (Game|SpawnActorfromClass "/Game/Assets/Blueprints/Milk.Milk_C" _returnvalue_6 "Undefined" 0 0)
              (elif (Math|Float|InRange(Float) _returnvalue_2 0.8 0.9)
                (Game|SpawnActorfromClass "/Game/Assets/Blueprints/ObstacleWall_Right.ObstacleWall_Right_C" _returnvalue_6 "Undefined" 0 0)
                (elif (Math|Float|InRange(Float) _returnvalue_2 0.9 0.95)
                  (Game|SpawnActorfromClass "/Game/Assets/Blueprints/ObstacleRocks.ObstacleRocks_C" _returnvalue_6 "Undefined" 0 0)
                  (elif (Math|Float|InRange(Float) _returnvalue_2 0.95 1.0)
                    (Game|SpawnActorfromClass "/Game/Assets/Blueprints/Magnet.Magnet_C" _returnvalue_6 "Undefined" 0 0))))))))
      (elif (Math|Float|InRange(Float) _returnvalue_3 0.3 0.5)
        (Game|SpawnActorfromClass "/Game/Assets/Blueprints/ObstacleBarrel.ObstacleBarrel_C" _returnvalue_5 "Undefined" 0 0)
        (Game|SpawnActorfromClass "/Game/Assets/Blueprints/CoinPickupJump.CoinPickupJump_C" _returnvalue_5 "Undefined" 0 0)
        (goto _label_2)
        (elif (Math|Float|InRange(Float) _returnvalue_3 0.5 0.7)
          (Game|SpawnActorfromClass "/Game/Assets/Blueprints/ObstacleBarrel.ObstacleBarrel_C" _returnvalue_5 "Undefined" 0 0)
          (goto _label_2)
          (elif (Math|Float|InRange(Float) _returnvalue_3 0.7 0.9)
            (Game|SpawnActorfromClass "/Game/Assets/Blueprints/Milk.Milk_C" _returnvalue_5 "Undefined" 0 0)
            (goto _label_2)
            (elif (Math|Float|InRange(Float) _returnvalue_3 0.9 0.95)
              (Game|SpawnActorfromClass "/Game/Assets/Blueprints/ObstacleRocks.ObstacleRocks_C" _returnvalue_5 "Undefined" 0 0)
              (goto _label_2)
              (elif (Math|Float|InRange(Float) _returnvalue_3 0.95 1.0)
                (Game|SpawnActorfromClass "/Game/Assets/Blueprints/Magnet.Magnet_C" _returnvalue_5 "Undefined" 0 0)
                (goto _label_2)))))))
    (elif (Math|Float|InRange(Float) _returnvalue 0.3 0.5)
      (Game|SpawnActorfromClass "/Game/Assets/Blueprints/ObstacleBarrel.ObstacleBarrel_C" _returnvalue_4 "Undefined" 0 0)
      (Game|SpawnActorfromClass "/Game/Assets/Blueprints/CoinPickupJump.CoinPickupJump_C" _returnvalue_4 "Undefined" 0 0)
      (goto _label)
      (elif (Math|Float|InRange(Float) _returnvalue 0.5 0.7)
        (Game|SpawnActorfromClass "/Game/Assets/Blueprints/ObstacleBarrel.ObstacleBarrel_C" _returnvalue_4 "Undefined" 0 0)
        (goto _label)
        (elif (Math|Float|InRange(Float) _returnvalue 0.7 0.8)
          (Game|SpawnActorfromClass "/Game/Assets/Blueprints/Milk.Milk_C" _returnvalue_4 "Undefined" 0 0)
          (goto _label)
          (elif (Math|Float|InRange(Float) _returnvalue 0.8 0.9)
            (Game|SpawnActorfromClass "/Game/Assets/Blueprints/ObstacleWall_Left.ObstacleWall_Left_C" _returnvalue_4 "Undefined" 0 0)
            (goto _label)
            (elif (Math|Float|InRange(Float) _returnvalue 0.9 0.95)
              (Game|SpawnActorfromClass "/Game/Assets/Blueprints/ObstacleRocks.ObstacleRocks_C" _returnvalue_4 "Undefined" 0 0)
              (goto _label)
              (elif (Math|Float|InRange(Float) _returnvalue 0.95 1.0)
                (Game|SpawnActorfromClass "/Game/Assets/Blueprints/Magnet.Magnet_C" _returnvalue_4 "Undefined" 0 0)
                (goto _label)))))))))